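; Base character Blueprint for MSGO with enhanced input, ability granting, hover-jump movement and enemy lock-on.
; Each Tick pushes movement and jump state to the Anim Blueprint.
; Lock-on picks the most screen-centered, recently rendered enemy by dot product, then turns the character, clamps camera angles and drives a HUD marker.
; Jumping rises to a height limit, then hovers with low gravity, falling back to a normal jump when overheated.
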(event `self.ReceiveBeginPlay`
  (bind _returnvalue (`GameplayStatics.GetPlayerCameraManager` 0))
  (bind _returnvalue_2 (`GameplayStatics.GetPlayerCameraManager` 0))
  (bind _returnvalue_3 (`SkeletalMeshComponent.GetAnimInstance` (`self.Mesh`)))
  (`EnhancedInputSubsystemInterface.AddMappingContext` (pcsubsystem `EnhancedInputLocalPlayerSubsystem` (`GameplayStatics.GetPlayerController` 0)) "/Game/Input/IMC_MSGO.IMC_MSGO" 0 (struct))
  (`/Engine/EditorBlueprintResources/StandardMacros.IsValid` _returnvalue_3
    (:`Is Valid`
      (set `self.AnimBP` _returnvalue_3)
      (set `self.SpawnPos` (`self.K2_GetActorLocation`))
      (set `self.ChracterName` (`KismetStringLibrary.Conv_StringToName` (`KismetStringLibrary.LeftChop` (`KismetSystemLibrary.GetDisplayName` self) 4)))
      (for _array_element (`self.AlibityList`)
        (`AbilitySystemComponent.K2_GiveAbility` (`self.AbilitySystem`) _array_element 0 -1)
        (set `PlayerCameraManager.ViewPitchMax` (`self.DefaultCameraPitchMax`) _returnvalue_2)
        (set `PlayerCameraManager.ViewPitchMin` (`self.DefaultCameraPitchMin`) _returnvalue_2)
        (set `self.DefaultCameraYawMax` (`PlayerCameraManager.ViewYawMax` _returnvalue))
        (set `self.DefaultCameraYawMin` (`PlayerCameraManager.ViewYawMin` _returnvalue))))))

(event `self.ReceiveTick`
  (params (DeltaSeconds :type "Float (single-precision)"))
  (bind (_returnvalue_roll _returnvalue_pitch _returnvalue_yaw) (`KismetMathLibrary.BreakRotator` (`self.K2_GetActorRotation`)))
  (bind (_defaultcamerarot_roll _defaultcamerarot_pitch) (`KismetMathLibrary.BreakRotator` (`self.DefaultCameraRot`)))
  (bind (_returnvalue_roll_2 _returnvalue_pitch_2 _returnvalue_yaw_2) (`KismetMathLibrary.BreakRotator` (`KismetMathLibrary.FindLookAtRotation` (`self.K2_GetActorLocation`) (`self.K2_GetActorLocation` (`self.TargetActor`)))))
  (bind (_returnvalue_roll_3 _returnvalue_pitch_3) (`KismetMathLibrary.BreakRotator` (`KismetMathLibrary.FindLookAtRotation` (`SceneComponent.K2_GetComponentLocation` (`self.FollowCamera`)) (`self.K2_GetActorLocation` (`self.TargetActor`)))))
  ;[1 1 1] ABPに移動速度を渡す
  (message `/Game/Characters/Common/BPI_AnimBPValue.SetMoveSpeed` (`self.AnimBP`) (`KismetMathLibrary.VSizeXY` (`MovementComponent.Velocity` (`self.CharacterMovement`))))
  (message `/Game/Characters/Common/BPI_AnimBPValue.SetMoveInput` (`self.AnimBP`) (`self.GetMoveInputVector`))
  (message `/Game/Characters/Common/BPI_AnimBPValue.SetIsDash` (`self.AnimBP`) (`self.MoveType`))
  (message `/Game/Characters/Common/BPI_AnimBPValue.SetFalling` (`self.AnimBP`) (`NavMovementComponent.IsFalling` (`self.CharacterMovement`)))
  (message `/Game/Characters/Common/BPI_AnimBPValue.SetJumpStatus` (`self.AnimBP`) (`self.NowJumpStatus`))
  (message `/Game/Characters/Common/BPI_AnimBPValue.SetMovementMode` (`self.AnimBP`) (`CharacterMovementComponent.MovementMode` (`self.CharacterMovement`)))
  (if (`self.bLockon`)
    (`self.K2_SetActorRotation` (`KismetMathLibrary.MakeRotator` 0.0 0.0 _returnvalue_yaw_2)) ; Z軸のみターゲットの方を向く
    (`self.SetCameraAngleLimit` true _returnvalue_yaw (- _returnvalue_pitch_3 _defaultcamerarot_pitch))
    (bind _outtarget2dpos (`self.GetTargetActor2DPos` (`self.K2_GetActorLocation` (`self.TargetActor`))))
    (`/Game/UI/Widget/WBP_MSGOHud.SetLockonMarkerPos` (`self.GetMSGOHud`) _outtarget2dpos)))

(event `EnhancedInput|/Game/Input/IA_LockOn`
  (params (ActionValue :type Boolean) (ElapsedSeconds :type "Float (double-precision)") (TriggeredSeconds :type "Float (double-precision)") (InputAction :type "InputAction Object Reference" :default "/Game/Input/IA_LockOn.IA_LockOn"))
  (:`Started`
    (`self.LockonCamera`)))

(event `LockonCamera`
  (bind (_returnvalue_roll _returnvalue_pitch _returnvalue_yaw) (`KismetMathLibrary.BreakRotator` (`self.K2_GetActorRotation`)))
  (bind _followcamera (`self.FollowCamera`))
  (bind (_defaultcamerarot_roll _defaultcamerarot_pitch) (`KismetMathLibrary.BreakRotator` (`self.DefaultCameraRot`)))
  (bind (_returnvalue_roll_2 _returnvalue_pitch_2 _returnvalue_yaw_2) (`KismetMathLibrary.BreakRotator` (`KismetMathLibrary.FindLookAtRotation` (`self.K2_GetActorLocation`) (`self.K2_GetActorLocation` (`self.TargetActor`)))))
  (bind (_returnvalue_roll_3 _returnvalue_pitch_3) (`KismetMathLibrary.BreakRotator` (`KismetMathLibrary.FindLookAtRotation` (`SceneComponent.K2_GetComponentLocation` (`self.FollowCamera`)) (`self.K2_GetActorLocation` (`self.TargetActor`)))))
  (if (`self.bLockon`)
    (set `self.bLockon` false)
    (set `self.TargetActor` null)
    (`self.SetCameraAngleLimit` false)
    (set `SpringArmComponent.bEnableCameraLag` true (`self.CameraBoom`))
    (`/Game/UI/Widget/WBP_MSGOHud.VisibleLockonMarker` (`self.GetMSGOHud`) false) ; ロックオンマーカー非表示
    (else
      (`|ExecutionSequence`
        (:`then_0`
          (bind _outactors (`GameplayStatics.GetAllActorsOfClassWithTag` "/Script/MSGO.MSGOCharacter" "Enemy"))
          (set `self.EnemyActors` _outactors)
          (for _array_element (`self.EnemyActors`)
            (bind _returnvalue (`KismetMathLibrary.Dot_VectorVector` (`KismetMathLibrary.Normal` (- (`self.K2_GetActorLocation` _array_element) (`SceneComponent.K2_GetComponentLocation` _followcamera))) (`SceneComponent.GetForwardVector` _followcamera)))
            (if (and (> _returnvalue (`self.TargetDotValue`)) (> _returnvalue 0.0) (`self.WasRecentlyRendered` _array_element 0.2))
              (set `self.TargetActor` _array_element)
              (set `self.TargetDotValue` _returnvalue)))
          (set `self.TargetDotValue` 0.0))
        (:`then_1`
          (`/Engine/EditorBlueprintResources/StandardMacros.IsValid` (`self.TargetActor`)
            (:`Is Valid`
              (set `self.bLockon` true)
              (`self.K2_SetActorRotation` (`KismetMathLibrary.MakeRotator` 0.0 0.0 _returnvalue_yaw_2)) ; Z軸のみターゲットの方を向く
              (`Controller.SetControlRotation` (`GameplayStatics.GetPlayerController` 0) (`KismetMathLibrary.MakeRotator` 0.0 (- _returnvalue_pitch_3 _defaultcamerarot_pitch) _returnvalue_yaw))
              (set `SpringArmComponent.bEnableCameraLag` false (`self.CameraBoom`))
              (`/Game/UI/Widget/WBP_MSGOHud.VisibleLockonMarker` (`self.GetMSGOHud`) true) ; ロックオンマーカー表示
            )))))))

(fn `Begin Jump`
  (bind (_returnvalue_x _returnvalue_y _returnvalue_z) (`KismetMathLibrary.BreakVector` (`self.K2_GetActorLocation`)))
  (if (not (`CharacterStatusComponent.GetIsOverHeat` (`self.StatusComponent`)))
    (switch `EJUMP_STATUS` (`self.NowJumpStatus`)
      (:`Idle`
        (set `self.BeginJumpHeght` _returnvalue_z)
        (set `self.NowJumpStatus` "Rising")
        (`CharacterMovementComponent.SetMovementMode` (`self.CharacterMovement`) "MOVE_Flying" 0))
      (:`Falling`
        (set `self.NowJumpStatus` "Hovering")
        (set `MovementComponent.Velocity` (0.0 0.0 0.0) (`self.CharacterMovement`))))
    (else
      (`self.Jump`))))

(fn `EndJump`
  (bind _nowjumpstatus (`self.NowJumpStatus`))
  (bind _charactermovement (`self.CharacterMovement`))
  (if (`|EnumInequality` (`self.MoveType`) "Dash")
    (if (or (`|EnumEquality` _nowjumpstatus "Rising") (`|EnumEquality` _nowjumpstatus "Hovering"))
      (`CharacterMovementComponent.SetMovementMode` _charactermovement "MOVE_Falling" 0)
      (set `CharacterMovementComponent.GravityScale` 1.0 _charactermovement)
      (set `self.NowJumpStatus` "Falling"))))

(fn `GetMoveInputVector`
  (returns (OutInputVector :type "Vector2D Structure"))
  (bind (_returnvalue_roll _returnvalue_pitch _returnvalue_yaw) (`KismetMathLibrary.BreakRotator` (`self.K2_GetActorRotation`)))
  (bind (_returnvalue_x _returnvalue_y) (`KismetMathLibrary.BreakVector` (`KismetMathLibrary.GreaterGreater_VectorRotator` (`MovementComponent.Velocity` (`self.GetMovementComponent`)) (`KismetMathLibrary.MakeRotator` 0.0 0.0 (* _returnvalue_yaw -1.0)))))
  (return (`KismetMathLibrary.Normal2D` (`KismetMathLibrary.MakeVector2D` _returnvalue_x _returnvalue_y))))

(fn `GetMSGOHud`
  (returns (NewParam :type "/Game/UI/Widget/WBP_MSGOHud Object Reference"))
  (bind _asmsgohud (cast `/Game/UI/HUD/MSGOHud` (`PlayerController.GetHUD` (`GameplayStatics.GetPlayerController` 0)))
    (:`then`
      (return (`/Game/UI/HUD/MSGOHud.UIRef` _asmsgohud)))
    (:`CastFailed`
      (return null))))

(fn `GetTargetActor2DPos`
  (params (InTargetPos :type "Vector Structure"))
  (returns (OutTarget2DPos :type "Vector2D Structure"))
  (return (/ (`PlayerController.ProjectWorldLocationToScreen` (`GameplayStatics.GetPlayerController` 0) (`local.InTargetPos`) false) (`WidgetLayoutLibrary.GetViewportScale`))))

(fn `IsHeightLimit`
  (returns (bIsHeightLimit :type Boolean))
  (bind (_returnvalue_x _returnvalue_y _returnvalue_z) (`KismetMathLibrary.BreakVector` (`self.K2_GetActorLocation`)))
  (return (>= (- _returnvalue_z (`self.BeginJumpHeght`)) (`.JumpRiseHeight` (break `CharacterStatusParameter` (`CharacterStatusComponent.StatusParameter` (`self.StatusComponent`)))))))

(fn `SetCameraAngleLimit`
  (params (bLockonCamera :type Boolean) (InPlayerYaw :type "Float (double-precision)") (InCameraPitch :type "Float (double-precision)"))
  (bind _returnvalue (`GameplayStatics.GetPlayerCameraManager` 0))
  (set `PlayerCameraManager.ViewPitchMax` (`KismetMathLibrary.SelectFloat` (+ (`local.InCameraPitch`) (`self.LockonPitchLimit`)) (`self.DefaultCameraPitchMax`) (`local.bLockonCamera`)) _returnvalue)
  (set `PlayerCameraManager.ViewPitchMin` (`KismetMathLibrary.SelectFloat` (- (`local.InCameraPitch`) (`self.LockonPitchLimit`)) (`self.DefaultCameraPitchMin`) (`local.bLockonCamera`)) _returnvalue)
  (set `PlayerCameraManager.ViewYawMax` (`KismetMathLibrary.SelectFloat` (+ (`local.InPlayerYaw`) (`self.LockonYawLimit`)) (`self.DefaultCameraYawMax`) (`local.bLockonCamera`)) _returnvalue)
  (set `PlayerCameraManager.ViewYawMin` (`KismetMathLibrary.SelectFloat` (- (`local.InPlayerYaw`) (`self.LockonYawLimit`)) (`self.DefaultCameraYawMin`) (`local.bLockonCamera`)) _returnvalue))

(fn `UpdateJump`
  (if (not (`CharacterStatusComponent.GetIsOverHeat` (`self.StatusComponent`)))
    (switch `EJUMP_STATUS` (`self.NowJumpStatus`)
      (:`Rising`
        (if (not (`self.IsHeightLimit`))
          (`self.K2_AddActorWorldOffset` (0.0 0.0 10.0))
          (else
            (set `self.NowJumpStatus` "Hovering"))))
      (:`Hovering`
        (`CharacterMovementComponent.SetMovementMode` (`self.CharacterMovement`) "MOVE_Falling" 0)
        (set `CharacterMovementComponent.GravityScale` 0.1 (`self.CharacterMovement`)))
      (:`Falling`
        (set `CharacterMovementComponent.GravityScale` 0.1 (`self.CharacterMovement`))))))

(fn `UserConstructionScript`
  (set `self.DefaultCameraRot` (`SceneComponent.RelativeRotation` (`self.FollowCamera`)))
  (`DamageCollision.SetupCollision` (`self.DamageCollision`) (make `DamageCollisionParameter` (32.0 32.0 80.0))))