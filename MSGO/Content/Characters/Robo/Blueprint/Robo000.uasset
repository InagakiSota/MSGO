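; Robo character Blueprint that drives emissive glow on its skeletal mesh and lights up its blade while the Attack input is held.
; BeginPlay creates dynamic material instances for two mesh material slots, one for body emissive and one for the blade.
; Tick calls Play on a timeline that animates the first material's EmissiveValue.
; Attack press and release switch the blade's EmissiveValue between bright and off, with no other attack logic here.
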(event `self.ReceiveBeginPlay`
  (`parent.ReceiveBeginPlay`)
  (bind _returnvalue (`PrimitiveComponent.CreateDynamicMaterialInstance` (`self.Mesh`) 3 null "None"))
  (set `self.MI_emissive` _returnvalue)
  (bind _returnvalue_2 (`PrimitiveComponent.CreateDynamicMaterialInstance` (`self.Mesh`) 1 null "None"))
  (set `self.MI_blade` _returnvalue_2))

(event `self.ReceiveTick`
  (params (DeltaSeconds :type "Float (single-precision)"))
  (`parent.ReceiveTick` DeltaSeconds)
  (bind (_direction _emissivevalue) (`Timeline|EmisiveTimeLine`)
    (:`Update`
      (`MaterialInstanceDynamic.SetScalarParameterValue` (`self.MI_emissive`) "EmissiveValue" _emissivevalue))))

(event `InputAction|Attack`
  (params (Key :type "Key Structure"))
  (bind _mi_blade (`self.MI_blade`))
  (:`Pressed`
    (`MaterialInstanceDynamic.SetScalarParameterValue` _mi_blade "EmissiveValue" 50.0))
  (:`Released`
    (`MaterialInstanceDynamic.SetScalarParameterValue` _mi_blade "EmissiveValue" 0.0)))

(fn `UserConstructionScript`)