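; Robo000 is a robot character Blueprint that adds glow feedback and attack aiming on top of its parent class.
; BeginPlay creates dynamic materials for the emissive and blade mesh slots, prints the MachineID, and plays a timeline driving emissive intensity.
; Tick tints the emissive red-orange when StatusComponent reports overheat, otherwise green.
; IA_Attack lights the blade and calls RotToCamera while triggered, then switches the glow off on completion.
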(event `self.ReceiveBeginPlay`
  (`parent.ReceiveBeginPlay`)
  (bind _returnvalue (`PrimitiveComponent.CreateDynamicMaterialInstance` (`self.Mesh`) 3 null "None"))
  (set `self.MI_emissive` _returnvalue)
  (bind _returnvalue_2 (`PrimitiveComponent.CreateDynamicMaterialInstance` (`self.Mesh`) 1 null "None"))
  (set `self.MI_blade` _returnvalue_2)
  (`KismetSystemLibrary.PrintString` (`KismetStringLibrary.Conv_IntToString` (`self.MachineID`)))
  (bind (_direction _emissivevalue) (`Timeline|タイムライン`)
    (:`Update`
      (`MaterialInstanceDynamic.SetScalarParameterValue` (`self.MI_emissive`) "EmissiveValue" _emissivevalue))))

(event `self.ReceiveActorBeginOverlap`
  (params (OtherActor :type "Actor Object Reference")))

(event `self.ReceiveTick`
  (params (DeltaSeconds :type "Float (single-precision)"))
  (`parent.ReceiveTick` DeltaSeconds)
  (`MaterialInstanceDynamic.SetVectorParameterValue` (`self.MI_emissive`) "EmissiveColor" (`KismetMathLibrary.SelectColor` (struct :`R` 1.0 :`G` 0.022204 :`A` 1.0) (struct :`G` 1.0 :`B` 0.119305 :`A` 1.0) (`CharacterStatusComponent.GetIsOverHeat` (`self.StatusComponent`)))))

(event `EnhancedInput|/Game/Input/IA_Attack`
  (params (ActionValue :type Boolean) (ElapsedSeconds :type "Float (double-precision)") (TriggeredSeconds :type "Float (double-precision)") (InputAction :type "InputAction Object Reference" :default "/Game/Input/IA_Attack.IA_Attack"))
  (bind _mi_blade (`self.MI_blade`))
  (:`Triggered`
    (`MaterialInstanceDynamic.SetScalarParameterValue` _mi_blade "EmissiveValue" 50.0)
    (`self.RotToCamera` (`self.YawRotSpeed`)))
  (:`Completed`
    (`MaterialInstanceDynamic.SetScalarParameterValue` _mi_blade "EmissiveValue" 0.0)))

(fn `UserConstructionScript`)